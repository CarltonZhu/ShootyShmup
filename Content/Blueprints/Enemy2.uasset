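; Enemy2 is an enemy actor that moves along negative world X each tick, with random speed and scale set at BeginPlay.
; Damage decrements health, triggering a material flash, brief shrink, sound and particles, restored from cached material and size.
; Death adds score through CarltonsPlayerController, then plays explosion effects and camera shake.
; Overlapping MyPawn costs player health and destroys the enemy; the random rotation values feed only an unconnected node.
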(event `self.ReceiveBeginPlay`
  (`self.SetInitialSpeed`)
  (`self.SetRandomScale`)
  (`self.SetRandomNess`)
  (`self.CachingMyMaterial`)
  (`self.CacheMyInitialSize`))

(event `self.ReceiveTick`
  (params (DeltaSeconds :type "Float (single-precision)"))
  ;[1 1 1] Move Forward
  (`self.K2_AddActorWorldOffset` (`KismetMathLibrary.MakeVector` (* (`self.speed`) -1.0)) true))

(event `Flash`
  ;[1 1 1] Flash
  (`PrimitiveComponent.SetMaterial` (`self.Cube`) 0 "/Game/Materials/Flash.Flash")
  (`self.SetActorScale3D` (* (`self.GetActorScale3D`) 0.8))
  (`KismetSystemLibrary.Delay` 0.1)
  (`PrimitiveComponent.SetMaterial` (`self.Cube`) 0 (`self.OgMaterial`))
  (`self.SetActorScale3D` (`self.InitialSize`)))

(event `self.ReceiveAnyDamage`
  (params (Damage :type "Float (single-precision)") (DamageType :type "DamageType Object Reference") (InstigatedBy :type "Controller Object Reference") (DamageCauser :type "Actor Object Reference"))
  ;[1 1 1] Health
  (bind _output_get (set `self.Health` (- (`self.Health`) 1.0)))
  (if (<= _output_get 0.0)
    (`self.DeathStuff`)
    (else
      (`self.Hit Feedback`))))

(event `DeathStuff`
  ;[1 0.8542 0.8542] Death Code
  (bind _ascarltons_player_controller (cast `/Game/Core/CarltonsPlayerController` (`GameplayStatics.GetPlayerController` 0)))
  (`/Game/Core/CarltonsPlayerController.AddingScore` _ascarltons_player_controller)
  (`GameplayStatics.PlaySound2D` "/Game/Sounds/explosion__1__Cue.explosion__1__Cue" 1.0 1.0 0.0 null null)
  (`GameplayStatics.SpawnEmitterAtLocation` "/Game/FXVarietyPack/Particles/P_ky_explosion.P_ky_explosion" (`self.K2_GetActorLocation`) (struct) (2.0 2.0 2.0))
  (`PlayerCameraManager.StartCameraShake` :`self` (`GameplayStatics.GetPlayerCameraManager` 0) :`ShakeClass` "/Game/Blueprints/Shakes/MyCameraShake.MyCameraShake_C" :`Scale` 300.0)
  (`self.K2_DestroyActor`))

(event `Hit Feedback`
  ;[1 0.7812 0.7812] Hit Feedback
  (`self.Flash`)
  (`GameplayStatics.PlaySound2D` "/Game/Sounds/hitHurt_Cue.hitHurt_Cue" 1.0 1.0 0.0 null null)
  (`GameplayStatics.SpawnEmitterAtLocation` "/Game/FXVarietyPack/Particles/P_ky_hit2.P_ky_hit2" (`self.K2_GetActorLocation`) (struct) (0.4 0.4 0.4)))

(event `self.SphereCOLLISION.OnComponentBeginOverlap`
  (params (OverlappedComponent :type "PrimitiveComponent Object Reference") (OtherActor :type "Actor Object Reference") (OtherComp :type "PrimitiveComponent Object Reference") (OtherBodyIndex :type Integer) (bFromSweep :type Boolean) (SweepResult :type "HitResult Structure (by ref)"))
  (cast `/Game/Blueprints/MyPawn` OtherActor)
  (bind _ascarltons_player_controller (cast `/Game/Core/CarltonsPlayerController` (`GameplayStatics.GetPlayerController` 0)))
  (`/Game/Core/CarltonsPlayerController.LoseHealth` _ascarltons_player_controller)
  (bind _asmy_pawn (cast `/Game/Blueprints/MyPawn` (`GameplayStatics.GetPlayerPawn` 0)))
  (`/Game/Blueprints/MyPawn.GotHit` _asmy_pawn)
  (`self.K2_DestroyActor`))

(fn `CacheMyInitialSize`
  (set `self.InitialSize` (`self.GetActorScale3D`)))

(fn `CachingMyMaterial`
  (set `self.OgMaterial` (`PrimitiveComponent.GetMaterial` (`self.Cube`) 0)))

(fn `Flashy`
  (bind _cube (`self.Cube`))
  (`PrimitiveComponent.SetMaterial` _cube 0 "/Game/Materials/Flash.Flash")
  (`PrimitiveComponent.SetMaterial` _cube 0 null))

(fn `SetInitialSpeed`
  (set `self.speed` (`KismetMathLibrary.RandomFloatInRange` 2.0 10.0)))

(fn `SetRandomNess`
  (set `self.randX` (`KismetMathLibrary.RandomFloatInRange` -6.0 6.0))
  (set `self.randY` (`KismetMathLibrary.RandomFloatInRange` -6.0 6.0))
  (set `self.randZ` (`KismetMathLibrary.RandomFloatInRange` -6.0 6.0)))

(fn `SetRandomScale`
  (`self.SetActorScale3D` (`KismetMathLibrary.MakeVector` (`KismetMathLibrary.RandomFloatInRange` 1.0 6.0) (`KismetMathLibrary.RandomFloatInRange` 1.0 6.0) (`KismetMathLibrary.RandomFloatInRange` 1.0 6.0))))

(fn `UserConstructionScript`)