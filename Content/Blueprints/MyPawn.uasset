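; MyPawn is a player-controlled plane pawn that slides sideways from horizontal input and banks into its movement.
; On BeginPlay it adds the IMC Enhanced Input mapping context, and the Hori action offsets the actor along the Y axis.
; Tick spins the Propeller and eases PlaneRoot's roll toward an angle proportional to the current Hori value with a short MoveComponentTo.
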(event `self.ReceiveBeginPlay`
  (`EnhancedInputSubsystemInterface.AddMappingContext` (pcsubsystem `EnhancedInputLocalPlayerSubsystem` (`GameplayStatics.GetPlayerController` 0)) "/Game/Core/Inputs/IMC.IMC" 0 (struct)))

(event `EnhancedInput|/Game/Core/Inputs/Hori`
  (params (ActionValue :type "Float (double-precision)") (ElapsedSeconds :type "Float (double-precision)") (TriggeredSeconds :type "Float (double-precision)") (InputAction :type "InputAction Object Reference" :default "/Game/Core/Inputs/Hori.Hori"))
  (:`Triggered`
    (`self.K2_AddActorWorldOffset` (`KismetMathLibrary.MakeVector` 0.0 (* ActionValue 10.0)))))

(event `self.ReceiveTick`
  (params (DeltaSeconds :type "Float (single-precision)"))
  (`SceneComponent.K2_AddRelativeRotation` (`self.Propeller`) (`KismetMathLibrary.MakeRotator` 10.0) false false)
  (`KismetSystemLibrary.MoveComponentTo` (`self.PlaneRoot`) (0.0 0.0 0.0) (`KismetMathLibrary.MakeRotator` (* (`|GetInputActionValue`) 45.0)) true true 0.06))

(fn `UserConstructionScript`)